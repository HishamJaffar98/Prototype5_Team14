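; Lava splash VFX example actor that plays a Niagara effect and keeps it looping.
; The construction script feeds NSScale into the Niagara component's User.GlobalScale.
; When that component finishes, it spawns an auto-release pooled PSN_Lava_Sparks_Surface at the actor's transform with the same scale, then binds its finish event to spawn again.
; The author notes that reactivating or re-initializing the system can crash, and advises against looping it.
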(event `self.ReceiveBeginPlay`)

(event `self.Niagara.OnSystemFinished`
  (params (PSystem :type "NiagaraComponent Object Reference"))
  (bind (_returnvalue_location _returnvalue_rotation _returnvalue_scale) (`KismetMathLibrary.BreakTransform` (`self.GetTransform`)))
  ;[1 1 1] Looping (DO NOT reactive or re-initialize, it can crash the game.  And I suggest not looping this NS)
  (bind _returnvalue (`NiagaraFunctionLibrary.SpawnSystemAtLocation` "/Game/VFX/Niagara_FX/ParticleSystems/PSN_Lava_Sparks_Surface.PSN_Lava_Sparks_Surface" _returnvalue_location _returnvalue_rotation _returnvalue_scale true true "AutoRelease" :!label _label))
  (`/Engine/EditorBlueprintResources/StandardMacros.IsValid` _returnvalue
    (:`Is Valid`
      (`FXSystemComponent.SetFloatParameter` _returnvalue "User.GlobalScale" (`self.NS_Scale`))
      (add `NiagaraComponent.OnSystemFinished` _returnvalue (delegate `OnSystemFinished_Event_0`)))))

(event `OnSystemFinished_Event_0`
  (params (PSystem :type "NiagaraComponent Object Reference"))
  ;[1 1 1] Looping (DO NOT reactive or re-initialize, it can crash the game.  And I suggest not looping this NS)
  (goto _label))

(fn `UserConstructionScript`
  (`NiagaraComponent.SetVariableFloat` (`self.Niagara`) "User.GlobalScale" (`self.NS_Scale`)))