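; Local multiplayer game mode that creates players and gives each an input receiver pawn before their character spawns.
; On BeginPlay it gathers PlayerStarts and, for each array index matching a numeric PlayerStartTag, creates a player and possesses a BP_InputReceiver.
; Receivers take the transform of the start at that array index, not of the tag-matched one.
; SpawnPlayer, not called here, spawns a ThirdPersonCharacter_1 at a receiver's transform and transfers possession to it.
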(event `self.ReceiveBeginPlay`
  (`self.GetPlayerStartPoints`)
  (`self.SpawnInputReceivers`))

(fn `GetPlayerStartPoints`
  (bind _outactors (`GameplayStatics.GetAllActorsOfClass` "/Script/Engine.PlayerStart"))
  (set `self.PlayerStartArray` _outactors))

(fn `NameToInt`
  (params (PlayerStart :type "PlayerStart Object Reference"))
  (returns (ReturnValue :type Integer))
  (return (`KismetStringLibrary.Conv_StringToInt` (`KismetStringLibrary.Conv_NameToString` (`PlayerStart.PlayerStartTag` PlayerStart)))))

(fn `SpawnInputReceivers`
  (locals (Index :type Integer))
  (bind _returnvalue (`GameplayStatics.GetPlayerController` (`local.Index`)))
  (for (_ _array_index) (`self.PlayerStartArray`)
    (set `local.Index` _array_index)
    (for _array_element (`self.PlayerStartArray`)
      (if (== (`self.NameToInt` _array_element) (`local.Index`))
        (`GameplayStatics.CreatePlayer` -1)
        (bind _returnvalue_2 (`|SpawnActorFromClass` "/Game/BP/Multiplayer/BP_InputReceiver.BP_InputReceiver_C" (`self.GetTransform` (`|GetArrayItem` (`self.PlayerStartArray`) (`local.Index`))) "Undefined" "OverrideRootScale" null (`local.Index`) null))
        (`KismetArrayLibrary.Array_AddUnique` (`self.PlayerInputReceiverArray`) _returnvalue_2)
        (`Controller.Possess` _returnvalue _returnvalue_2)
        (`KismetArrayLibrary.Array_AddUnique` (`self.PlayerControllerArray`) _returnvalue)))))

(fn `SpawnPlayer`
  (params (CurrentPlayerIndex :type Integer) (InputReceiver :type "/Game/BP/Multiplayer/BP_InputReceiver Object Reference"))
  (returns (Return :type Boolean))
  (bind _returnvalue (`|SpawnActorFromClass` "/Game/MountAndDash/ThirdPersonBP/Blueprints/ThirdPersonCharacter_1.ThirdPersonCharacter_1_C" (`self.GetTransform` (`local.InputReceiver`)) "Undefined" "OverrideRootScale" null (`local.CurrentPlayerIndex`) null))
  (`Controller.Possess` (`GameplayStatics.GetPlayerController` (`local.CurrentPlayerIndex`)) _returnvalue)
  (return false))

(fn `UserConstructionScript`)