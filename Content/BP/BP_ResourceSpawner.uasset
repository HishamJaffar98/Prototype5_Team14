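; BP_ResourceSpawner is an actor that scatters resource clusters inside a box volume when play begins.
; On BeginPlay it spawns a random number of BP_ResourceCluster actors between its minimum and maximum settings.
; Each cluster is placed at a random point within the Box extent around the root's world location, then attached to the spawner keeping its world transform.
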(event `self.ReceiveBeginPlay`
  (for _ (range 1 (+ (`KismetMathLibrary.RandomIntegerInRange` (`self.minClustersToSpawn`) (`self.maxClustersToSpawn`)) 1))
    (bind _returnvalue (`|SpawnActorFromClass` "/Game/BP/BP_ResourceCluster.BP_ResourceCluster_C" (`KismetMathLibrary.MakeTransform` (`KismetMathLibrary.RandomPointInBoundingBox` (`SceneComponent.K2_GetComponentLocation` (`self.DefaultSceneRoot`)) (`BoxComponent.BoxExtent` (`self.Box`)))) "Undefined" "OverrideRootScale" null null))
    (`/Engine/EditorBlueprintResources/StandardMacros.IsValid` _returnvalue
      (:`Is Valid`
        (`self.K2_AttachToActor` _returnvalue self "None" "KeepWorld" "KeepWorld" "KeepWorld" true)))))

(fn `UserConstructionScript`)