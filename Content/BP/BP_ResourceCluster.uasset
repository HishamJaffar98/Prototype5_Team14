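; BP_ResourceCluster is a group of resource pickups that respawns elsewhere once depleted.
; On BeginPlay it spawns a random number of pickups inside its box, attaches them to itself and caches the BP_ResourceSpawner.
; When an overlap with the box ends and no attached actors remain, it waits out a respawn delay.
; It then spawns a replacement cluster at a random point in the spawner's box, attaches it there and destroys itself.
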(event `self.ReceiveBeginPlay`
  (`|ExecutionSequence`
    (:`then_0`
      (for _ (range 1 (+ (`KismetMathLibrary.RandomIntegerInRange` (`self.minResourcesToSpawn`) (`self.maxResourcesToSpawn`)) 1))
        (bind _returnvalue (`|SpawnActorFromClass` "/Game/BP/ResourcePickup.ResourcePickup_C" (`KismetMathLibrary.MakeTransform` (`KismetMathLibrary.RandomPointInBoundingBox` (`SceneComponent.K2_GetComponentLocation` (`self.DefaultSceneRoot`)) (`BoxComponent.BoxExtent` (`self.Box`)))) "Undefined" "OverrideRootScale" null null))
        (`/Engine/EditorBlueprintResources/StandardMacros.IsValid` _returnvalue
          (:`Is Valid`
            (`self.K2_AttachToActor` _returnvalue self "None" "KeepWorld" "KeepWorld" "KeepWorld" true)))))
    (:`then_1`
      (bind _returnvalue_2 (`GameplayStatics.GetActorOfClass` "/Game/BP/BP_ResourceSpawner.BP_ResourceSpawner_C"))
      (set `self.resourceSpawner` _returnvalue_2))))

(event `self.Box.OnComponentEndOverlap`
  (params (OverlappedComponent :type "PrimitiveComponent Object Reference") (OtherActor :type "Actor Object Reference") (OtherComp :type "PrimitiveComponent Object Reference") (OtherBodyIndex :type Integer))
  (bind _resourcespawner (`self.resourceSpawner`))
  (if (== 0 (`KismetArrayLibrary.Array_Length` (`self.GetAttachedActors` true)))
    (`KismetSystemLibrary.PrintString` "NoChildren")
    (`KismetSystemLibrary.Delay` (`self.respawnDuration`))
    (bind _returnvalue (`|SpawnActorFromClass` "BP_ResourceCluster_C" (`KismetMathLibrary.MakeTransform` (`KismetMathLibrary.RandomPointInBoundingBox` (`SceneComponent.K2_GetComponentLocation` (`/Game/BP/BP_ResourceSpawner.DefaultSceneRoot` _resourcespawner)) (`BoxComponent.BoxExtent` (`/Game/BP/BP_ResourceSpawner.Box` _resourcespawner)))) "Undefined" "OverrideRootScale" null null))
    (`/Engine/EditorBlueprintResources/StandardMacros.IsValid` _returnvalue
      (:`Is Valid`
        (`self.K2_AttachToActor` _returnvalue (`self.resourceSpawner`) "None" "KeepWorld" "KeepWorld" "KeepWorld" true)
        (`self.K2_DestroyActor`)))))

(fn `UserConstructionScript`)