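; ResourcePickup is a pickup actor that bobs its mesh up and down continuously; the file shows no collection logic.
; On BeginPlay, a custom event chains two short latent MoveComponentTo calls, then calls itself to loop without using Tick.
; MoveUp and MoveDown supply the targets by adding or subtracting MoveOffset on the mesh's current relative Z, keeping X, Y and rotation unchanged.
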(event `self.ReceiveBeginPlay`
  (`self.AnimateResourcePickup`))

(event `AnimateResourcePickup`
  (bind _mesh (`self.Mesh`))
  (bind (_newposition _newrotation) (`self.MoveUp` _mesh))
  (`KismetSystemLibrary.MoveComponentTo` _mesh _newposition _newrotation false false 0.2)
  (bind (_newposition_2 _newrotation_2) (`self.MoveDown` _mesh))
  (`KismetSystemLibrary.MoveComponentTo` _mesh _newposition_2 _newrotation_2 false false 0.2)
  (`self.AnimateResourcePickup`))

(fn `MoveDown`
  (params (Mesh :type "StaticMeshComponent Object Reference"))
  (returns (NewPosition :type "Vector Structure") (NewRotation :type "Rotator Structure"))
  (bind (_relativelocation_x _relativelocation_y _relativelocation_z) (`KismetMathLibrary.BreakVector` (`SceneComponent.RelativeLocation` Mesh)))
  (return (`KismetMathLibrary.MakeVector` _relativelocation_x _relativelocation_y (- _relativelocation_z (`self.moveOffset`))) (`SceneComponent.RelativeRotation` Mesh)))

(fn `MoveUp`
  (params (Mesh :type "StaticMeshComponent Object Reference"))
  (returns (NewPosition :type "Vector Structure") (NewRotation :type "Rotator Structure"))
  (bind (_relativelocation_x _relativelocation_y _relativelocation_z) (`KismetMathLibrary.BreakVector` (`SceneComponent.RelativeLocation` Mesh)))
  (return (`KismetMathLibrary.MakeVector` _relativelocation_x _relativelocation_y (+ _relativelocation_z (`self.moveOffset`))) (`SceneComponent.RelativeRotation` Mesh)))

(fn `UserConstructionScript`)