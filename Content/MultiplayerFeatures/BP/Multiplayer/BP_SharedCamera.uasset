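; BP_SharedCamera is a shared multiplayer camera that follows the group of active players once GameStarted hands it their list.
; Each tick, MoveCamera lerps the Sphere component toward the players' average location, using CameraMoveSpeed as a per-tick alpha.
; Tick also gathers distances between players and sets the spring arm length to the largest, clamped between minimum and maximum camera size.
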(event `self.ReceiveTick`
  (params (DeltaSeconds :type "Float (single-precision)"))
  (if (`self.bGameStarted`)
    (`self.MoveCamera`)
    (for (_array_element _array_index) (`self.Active Players`)
      (set `self.CurrentPlayer` _array_element)
      (for _index (range (+ _array_index 1) (+ (- 0 (`KismetArrayLibrary.Array_Length` (`self.Active Players`))) 1))
        (`KismetArrayLibrary.Array_Add` (`self.Distance`) (`self.GetDistanceTo` (`self.CurrentPlayer`) null))))
    (set `SpringArmComponent.TargetArmLength` (`KismetMathLibrary.FClamp` (`.MaxValue` (`KismetMathLibrary.MaxOfFloatArray` (`self.Distance`))) (`self.MinimumCameraSize`) (`self.MaximumCameraSize`)) (`self.SpringArm`))
    (`KismetArrayLibrary.Array_Clear` (`self.Distance`))))

(fn `GameStarted`
  (params (ActivePlayers :type "Array of /Game/BP/ThirdPersonCharacter_1 Object Reference"))
  (set `self.Active Players` ActivePlayers)
  (set `self.bGameStarted` true))

(fn `MoveCamera`
  (set `self.PreviousLocation` (`SceneComponent.K2_GetComponentLocation` (`self.Sphere`)))
  (bind _returnvalue (`GameplayStatics.GetActorArrayAverageLocation` (`self.Active Players`)))
  (`SceneComponent.K2_SetWorldLocation` (`self.Sphere`) (`KismetMathLibrary.VLerp` (`self.PreviousLocation`) _returnvalue (`self.CameraMoveSpeed`)) false false))

(fn `UserConstructionScript`)