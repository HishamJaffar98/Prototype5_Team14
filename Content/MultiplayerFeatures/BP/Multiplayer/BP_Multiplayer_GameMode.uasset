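; Local multiplayer game mode that creates a player for each tagged PlayerStart and shares one BP_SharedCamera view.
; BeginPlay orders starts by numeric tag, possesses a BP_InputReceiver at each, and destroys CameraActors.
; SpawnPlayer later spawns and possesses a BP_ThirdPersonBall at a receiver's position, adding it to Players.
; StartGame calls GameStarted when MinimumPlayers >= player count, setting the in-game flag and passing Players to the camera.
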(event `self.ReceiveBeginPlay`
  (bind _outactors (`GameplayStatics.GetAllActorsOfClass` "/Game/MultiplayerFeatures/BP/Multiplayer/BP_SharedCamera.BP_SharedCamera_C"))
  (set `self.CameraRef` (`|GetArrayItem` _outactors))
  (`self.GetPlayerStartPoints`)
  (`self.SpawnInputReceivers`))

(fn `GameStarted`
  (set `self.bIsInGame` true)
  (`/Game/MultiplayerFeatures/BP/Multiplayer/BP_SharedCamera.GameStarted` (`self.CameraRef`) (`self.Players`))
  (`KismetSystemLibrary.PrintString` "Hello"))

(fn `GetIsInGame`
  (returns (IsInGame :type Boolean))
  (return (`self.bIsInGame`)))

(fn `GetPlayerStartPoints`
  (bind _outactors (`GameplayStatics.GetAllActorsOfClass` "/Script/Engine.PlayerStart"))
  (bind _output_get (set `self.PlayerStartArray` _outactors))
  (`KismetSystemLibrary.PrintString` (`KismetStringLibrary.Conv_IntToString` (`KismetArrayLibrary.Array_Length` _output_get))))

(fn `NameToInt`
  (params (PlayerStart :type "PlayerStart Object Reference"))
  (returns (ReturnValue :type Integer))
  (return (`KismetStringLibrary.Conv_StringToInt` (`KismetStringLibrary.Conv_NameToString` (`PlayerStart.PlayerStartTag` PlayerStart)))))

(fn `RemoveUnusedCameras`
  (bind _outactors (`GameplayStatics.GetAllActorsOfClass` "/Script/Engine.CameraActor"))
  (for _array_element _outactors
    (`self.K2_DestroyActor` _array_element)))

(fn `SpawnInputReceivers`
  (locals (Index :type Integer))
  (bind _returnvalue (`GameplayStatics.GetPlayerController` (`local.Index`)))
  (for (_ _array_index) (`self.PlayerStartArray`)
    (set `local.Index` _array_index)
    (for _array_element (`self.PlayerStartArray`)
      (if (== (`self.NameToInt` _array_element) (`local.Index`))
        (`GameplayStatics.CreatePlayer` -1)
        (bind _returnvalue_2 (`|SpawnActorFromClass` "/Game/MultiplayerFeatures/BP/Multiplayer/BP_InputReceiver.BP_InputReceiver_C" (`self.GetTransform` (`|GetArrayItem` (`self.PlayerStartArray`) (`local.Index`))) "Undefined" "OverrideRootScale" null (`local.Index`) null))
        (`KismetArrayLibrary.Array_AddUnique` (`self.PlayerInputReceiverArray`) _returnvalue_2)
        (`Controller.Possess` _returnvalue _returnvalue_2)
        (`KismetArrayLibrary.Array_AddUnique` (`self.PlayerControllerArray`) _returnvalue)
        (`PlayerController.SetViewTargetWithBlend` (`GameplayStatics.GetPlayerController` (`local.Index`)) (`self.CameraRef`) 0.0 "VTBlend_Linear" 0.0 false)))
    (`self.RemoveUnusedCameras`)))

(fn `SpawnPlayer`
  (params (CurrentPlayerIndex :type Integer) (InputReceiver :type "/Game/MultiplayerFeatures/BP/Multiplayer/BP_InputReceiver Object Reference"))
  (returns (Return :type Boolean))
  (locals (InputReciever :type "/Game/MultiplayerFeatures/BP/Multiplayer/BP_InputReceiver Object Reference"))
  (bind _returnvalue (`|SpawnActorFromClass` "/Game/BP/BP_ThirdPersonBall.BP_ThirdPersonBall_C" (`self.GetTransform` InputReceiver) "Undefined" "OverrideRootScale" null (`local.CurrentPlayerIndex`) null))
  (`KismetArrayLibrary.Array_Add` (`self.Players`) _returnvalue)
  (`Controller.Possess` (`GameplayStatics.GetPlayerController` (`local.CurrentPlayerIndex`)) _returnvalue)
  (`PlayerController.SetViewTargetWithBlend` (`GameplayStatics.GetPlayerController` (`local.CurrentPlayerIndex`)) (`self.CameraRef`) 0.0 "VTBlend_Linear" 0.0 false)
  (return false))

(fn `StartGame`
  (returns (Return :type Boolean))
  (locals (MinimumPlayers :type Integer :default 2))
  (if (>= (`local.MinimumPlayers`) (`KismetArrayLibrary.Array_Length` (`self.Players`)))
    (`self.GameStarted`)
    (return true)))

(fn `UserConstructionScript`)